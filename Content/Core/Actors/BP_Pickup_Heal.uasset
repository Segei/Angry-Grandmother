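; BP_Pickup_Heal is a health pickup that heals whatever actor overlaps it, provided that actor implements HealingInterface.
; On overlap it passes a random amount between MinimalHeal and MaximalHeal through the interface, plays a pickup sound at its location and destroys itself.
; While it exists, it spins by a fixed world-rotation step every Tick, independent of delta time.
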(event `self.ReceiveActorBeginOverlap`
  (params (OtherActor :type "Actor Object Reference"))
  (bind _ashealing_interface (cast `HealingInterface` OtherActor))
  (`HealingInterface.TakeHealing` _ashealing_interface (`KismetMathLibrary.Lerp` (`self.MinimalHeal`) (`self.MaximalHeal`) (`KismetMathLibrary.RandomFloat`)))
  (`GameplayStatics.PlaySoundAtLocation` "/Game/Core/Sound/Heal_get.Heal_get" (`self.K2_GetActorLocation`) (struct) 1.0 1.0 0.0 null null null null)
  (`self.K2_DestroyActor`))

(event `self.ReceiveTick`
  (params (DeltaSeconds :type "Float (single-precision)"))
  (`self.K2_AddActorWorldRotation` (struct :`Yaw` 1.0)))

(fn `UserConstructionScript`)